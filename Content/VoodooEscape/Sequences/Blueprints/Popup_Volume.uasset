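; Popup_Volume is a trigger box that shows a timed dialogue popup when the ThirdPersonCharacter enters it.
; On overlap, a DoOnce gate creates or reuses a Dialogue_Box widget and fills it with the volume's left and right character images, names and message.
; A retriggerable delay hides the popup after the configured duration, then reopens the gate if ResetPopup is set.
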(event OnComponentBeginOverlap(Box)
  (params (OverlappedComponent :type Primitive%20Component%20Object%20Reference) (OtherActor :type Actor%20Object%20Reference) (OtherComp :type Primitive%20Component%20Object%20Reference) (OtherBodyIndex :type Integer) (bFromSweep :type Boolean) (SweepResult :type Hit%20Result%20Structure%20%28by%20ref%29))
  (if (== (Utilities|GetClass OtherActor) "/Game/ThirdPersonBP/Blueprints/ThirdPersonCharacter.ThirdPersonCharacter_C")
    (Utilities|FlowControl|DoOnce false
      (:Completed
        (Utilities|IsValid (Variables|Default|GetPopup)
          (:Is%20Valid
            (Widget|SetVisibility (Variables|Default|GetPopup) "Visible"))
          (:Is%20Not%20Valid
            (bind _returnvalue (UserInterface|CreateWidget "/Game/VoodooEscape/Sequences/Blueprints/Dialogue_Box.Dialogue_Box_C" (Game|GetPlayerController 0)))
            (bind _output_get (Variables|Default|SetPopup _returnvalue))
            (UserInterface|Viewport|AddtoViewport _output_get 0)
            (Widget|SetVisibility _output_get "Visible")))
        (CallFunction|PopupSettings)
        (Utilities|FlowControl|RetriggerableDelay (Variables|Default|GetDurration))
        (Widget|SetVisibility (Variables|Default|GetPopup) "Hidden")
        (if (Variables|Default|GetResetPopup)
          (CallFunction|Reset))))))

(event Custom|Reset
  (Utilities|FlowControl|DoOnce false) ; enters at Reset
)

(event Custom|Popup_Settings
  (bind _popup (Variables|Default|GetPopup))
  (Variables|/Game/VoodooEscape/Sequences/Blueprints/Dialogue_Box.Dialogue_Box_C|SetCharacterImage_Left _popup (Variables|Default|GetCharacterImage_Left))
  (Variables|/Game/VoodooEscape/Sequences/Blueprints/Dialogue_Box.Dialogue_Box_C|SetCharacterName_Left _popup (Variables|Default|GetCharacterName_Left))
  (Variables|/Game/VoodooEscape/Sequences/Blueprints/Dialogue_Box.Dialogue_Box_C|SetCharacterImage_Right _popup (Variables|Default|GetCharacterImage_Right))
  (Variables|/Game/VoodooEscape/Sequences/Blueprints/Dialogue_Box.Dialogue_Box_C|SetCharacterName_Right _popup (Variables|Default|GetCharacterName_Right))
  (Variables|/Game/VoodooEscape/Sequences/Blueprints/Dialogue_Box.Dialogue_Box_C|SetMessage _popup (Variables|Default|GetMessage)))

(event EventBeginPlay)

(event Collision|EventActorBeginOverlap
  (params (OtherActor :type Actor%20Object%20Reference)))

(event EventTick
  (params (DeltaSeconds :type Float%20%28single-precision%29)))

(fn ConstructionScript)