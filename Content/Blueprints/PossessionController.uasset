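; PossessionController is a controller Blueprint that uses the Tab key to toggle possession, tracked by a Possessed flag.
; When the flag is set, it possesses the first ThirdPersonCharacter found in the level.
; The opposite branch is unfinished, with no actor class or Possess target connected.
; A separate FaceForward function, not called here, passes the player character's location to SetInitialLocationAndRotation.
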(event EventBeginPlay)

(event EventTick
  (params (DeltaSeconds :type Float%20%28single-precision%29)))

(event Input|KeyboardEvents|Tab
  (params (Key :type Key%20Structure :default "AnyKey"))
  (:Pressed
    (if (Variables|Default|GetPossessed)
      (bind _outactors (Actor|GetAllActorsOfClass "/Game/ThirdPersonBP/Blueprints/ThirdPersonCharacter.ThirdPersonCharacter_C"))
      (Pawn|Possess (Utilities|Array|Get(acopy) _outactors))
      (Variables|Default|SetPossessed false)
      (else
        (bind _outactors_2 (Actor|GetAllActorsOfClass 0))
        (Pawn|Possess)
        (Variables|Default|SetPossessed true)))))

(fn ConstructionScript)

(fn FaceForward
  (Actor|GetAllActorsOfClass "/Game/ThirdPersonBP/Blueprints/ThirdPersonCharacter.ThirdPersonCharacter_C")
  (Class|Controller|SetInitialLocationandRotation (Transformation|GetActorLocation (Game|GetPlayerCharacter 0)) (Math|Rotator|MakeRotator 0.0 0.0 0.0)))